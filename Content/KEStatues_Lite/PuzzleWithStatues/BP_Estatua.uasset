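; Two-statue rotation puzzle actor that counts as solved when both Roman statues are aligned with their activators.
; Player overlap enables input and opens that statue's gate, so Interact plays a timeline rotating it by AngleRotation in yaw, with input locked during the turn.
; Puzzle triggers flag each statue while overlapping BP_ActivadorEstatuas.
; A looping timer polls both flags and only prints the result; the key spawn is unconnected.
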(event `PuzzleResuelto`
  (if (and (`self.Estatua1Activada`) (`self.Estatua2Activada`))
    (`KismetSystemLibrary.PrintString` "PuzzleResuelto")
    (else
      (`KismetSystemLibrary.PrintString` "PuzzleNOResuelto"))))

(event `self.ReceiveBeginPlay`
  (`|ExecutionSequence`
    (:`then_0`
      (set `self.GetCurrentRotationOfEstatua1` (`SceneComponent.K2_GetComponentRotation` (`self.EstatuaRomano1`)))
      (set `self.CurrentRotationEstatua2` (`SceneComponent.K2_GetComponentRotation` (`self.EstatuaRomano2`))))
    (:`then_1`
      (`KismetSystemLibrary.K2_SetTimer` null "PuzzleResuelto" 0.25 true))))

(event `EnhancedInput|/Game/ThirdPerson/Input/Actions/IA_Interact`
  (params (ActionValue :type Boolean) (ElapsedSeconds :type "Float (double-precision)") (TriggeredSeconds :type "Float (double-precision)") (InputAction :type "InputAction Object Reference" :default "/Game/ThirdPerson/Input/Actions/IA_Interact.IA_Interact"))
  (bind _returnvalue (`GameplayStatics.GetPlayerController` 0))
  (:`Triggered`
    (`/Engine/EditorBlueprintResources/StandardMacros.Gate` true :!label _label
      (:`Exit`
        (`self.DisableInput` _returnvalue)
        (bind (_direction _time) (`Timeline|TimelineEstatua1` :!via `PlayFromStart`)
          (:`Update`
            (bind _returnvalue_2 (`KismetMathLibrary.RLerp` (`self.GetCurrentRotationOfEstatua1`) (`KismetMathLibrary.MakeRotator` (.roll (`self.GetCurrentRotationOfEstatua1`)) (.pitch (`self.GetCurrentRotationOfEstatua1`)) (+ (.yaw (`self.GetCurrentRotationOfEstatua1`)) (`self.AngleRotation`))) _time))
            (`SceneComponent.K2_SetRelativeRotation` (`self.EstatuaRomano1`) _returnvalue_2 false false))
          (:`Finished`
            (set `self.GetCurrentRotationOfEstatua1` _returnvalue_2)
            (`self.EnableInput` _returnvalue)))))))

(event `self.TriggerActivatorEstatua.OnComponentBeginOverlap`
  (params (OverlappedComponent :type "PrimitiveComponent Object Reference") (OtherActor :type "Actor Object Reference") (OtherComp :type "PrimitiveComponent Object Reference") (OtherBodyIndex :type Integer) (bFromSweep :type Boolean) (SweepResult :type "HitResult Structure (by ref)"))
  (cast `/Game/ThirdPerson/Blueprints/BP_ThirdPersonCharacter` OtherActor)
  (`self.EnableInput` (`GameplayStatics.GetPlayerController` 0))
  (goto _label :!via `Open`))

(event `self.TriggerActivatorEstatua.OnComponentEndOverlap`
  (params (OverlappedComponent :type "PrimitiveComponent Object Reference") (OtherActor :type "Actor Object Reference") (OtherComp :type "PrimitiveComponent Object Reference") (OtherBodyIndex :type Integer))
  (cast `/Game/ThirdPerson/Blueprints/BP_ThirdPersonCharacter` OtherActor)
  (`self.DisableInput` (`GameplayStatics.GetPlayerController` 0))
  (goto _label :!via `Close`))

(event `self.TriggerActivadorPuzzle.OnComponentBeginOverlap`
  (params (OverlappedComponent :type "PrimitiveComponent Object Reference") (OtherActor :type "Actor Object Reference") (OtherComp :type "PrimitiveComponent Object Reference") (OtherBodyIndex :type Integer) (bFromSweep :type Boolean) (SweepResult :type "HitResult Structure (by ref)"))
  (cast `/Game/KEStatues_Lite/PuzzleWithStatues/BP_ActivadorEstatuas` OtherActor)
  (set `self.Estatua1Activada` true))

(event `self.TriggerActivadorPuzzle.OnComponentEndOverlap`
  (params (OverlappedComponent :type "PrimitiveComponent Object Reference") (OtherActor :type "Actor Object Reference") (OtherComp :type "PrimitiveComponent Object Reference") (OtherBodyIndex :type Integer))
  (cast `/Game/KEStatues_Lite/PuzzleWithStatues/BP_ActivadorEstatuas` OtherActor)
  (set `self.Estatua1Activada` false))

(event `EnhancedInput|/Game/ThirdPerson/Input/Actions/IA_Interact`
  (params (ActionValue :type Boolean) (ElapsedSeconds :type "Float (double-precision)") (TriggeredSeconds :type "Float (double-precision)") (InputAction :type "InputAction Object Reference" :default "/Game/ThirdPerson/Input/Actions/IA_Interact.IA_Interact"))
  (bind _returnvalue (`GameplayStatics.GetPlayerController` 0))
  (:`Triggered`
    (`/Engine/EditorBlueprintResources/StandardMacros.Gate` true :!label _label_2
      (:`Exit`
        (`self.DisableInput` _returnvalue)
        (bind (_direction _time) (`Timeline|Timeline` :!via `PlayFromStart`)
          (:`Update`
            (bind _returnvalue_2 (`KismetMathLibrary.RLerp` (`self.CurrentRotationEstatua2`) (`KismetMathLibrary.MakeRotator` (.roll (`self.CurrentRotationEstatua2`)) (.pitch (`self.CurrentRotationEstatua2`)) (+ (.yaw (`self.CurrentRotationEstatua2`)) (`self.AngleRotation`))) _time))
            (`SceneComponent.K2_SetRelativeRotation` (`self.EstatuaRomano2`) _returnvalue_2 false false))
          (:`Finished`
            (set `self.CurrentRotationEstatua2` _returnvalue_2)
            (`self.EnableInput` _returnvalue)))))))

(event `self.TriggerActivatorEstatua2.OnComponentBeginOverlap`
  (params (OverlappedComponent :type "PrimitiveComponent Object Reference") (OtherActor :type "Actor Object Reference") (OtherComp :type "PrimitiveComponent Object Reference") (OtherBodyIndex :type Integer) (bFromSweep :type Boolean) (SweepResult :type "HitResult Structure (by ref)"))
  (cast `/Game/ThirdPerson/Blueprints/BP_ThirdPersonCharacter` OtherActor)
  (`self.EnableInput` (`GameplayStatics.GetPlayerController` 0))
  (goto _label_2 :!via `Open`))

(event `self.TriggerActivatorEstatua2.OnComponentEndOverlap`
  (params (OverlappedComponent :type "PrimitiveComponent Object Reference") (OtherActor :type "Actor Object Reference") (OtherComp :type "PrimitiveComponent Object Reference") (OtherBodyIndex :type Integer))
  (cast `/Game/ThirdPerson/Blueprints/BP_ThirdPersonCharacter` OtherActor)
  (`self.DisableInput` (`GameplayStatics.GetPlayerController` 0))
  (goto _label_2 :!via `Close`))

(event `self.TriggerActivadorPuzzle2.OnComponentBeginOverlap`
  (params (OverlappedComponent :type "PrimitiveComponent Object Reference") (OtherActor :type "Actor Object Reference") (OtherComp :type "PrimitiveComponent Object Reference") (OtherBodyIndex :type Integer) (bFromSweep :type Boolean) (SweepResult :type "HitResult Structure (by ref)"))
  (cast `/Game/KEStatues_Lite/PuzzleWithStatues/BP_ActivadorEstatuas` OtherActor)
  (set `self.Estatua2Activada` true))

(event `self.TriggerActivadorPuzzle2.OnComponentEndOverlap`
  (params (OverlappedComponent :type "PrimitiveComponent Object Reference") (OtherActor :type "Actor Object Reference") (OtherComp :type "PrimitiveComponent Object Reference") (OtherBodyIndex :type Integer))
  (cast `/Game/KEStatues_Lite/PuzzleWithStatues/BP_ActivadorEstatuas` OtherActor)
  (set `self.Estatua2Activada` false))

(fn `UserConstructionScript`)